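; Hex-grid board actor for a link-three puzzle: spawns hex fields with randomly typed sphere meshes on BeginPlay.
; Selection chains adjacent same-type fields using column-parity neighbor masks, draws instanced bridges between them, and supports backtracking.
; Ending a chain of three or more empties those fields and notifies the player controller.
; Changes then drops pieces by instantly swapping per-column over gaps and refills empties with random types.
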(event `self.ReceiveBeginPlay`
  (`self.SpawnBoard`))

(fn `addBridge`
  (params (indexFrom :type Integer) (indexTo :type Integer))
  (bind _fieldsmeshes (`self.fieldsMeshes`))
  (bind _relativelocation (`SceneComponent.RelativeLocation` (`|GetArrayItem` _fieldsmeshes indexFrom)))
  (bind _relativelocation_2 (`SceneComponent.RelativeLocation` (`|GetArrayItem` _fieldsmeshes indexTo)))
  (`InstancedStaticMeshComponent.AddInstance` (`self.Bridges`) (`KismetMathLibrary.MakeTransform` (+ _relativelocation (* (`KismetMathLibrary.GetDirectionUnitVector` _relativelocation _relativelocation_2) 120.0) (0.0 0.0 30.0)) (`KismetMathLibrary.FindLookAtRotation` _relativelocation _relativelocation_2)))
  (return))

(fn `addField`
  (params (x :type Integer) (y :type Integer))
  (bind _index (`self.xy->index` x y))
  (set `self.lastX` x)
  (set `self.lastY` y)
  (`KismetArrayLibrary.Array_Add` (`self.selectedIndexes`) _index)
  (`/HexBlocksGame/hexFieldBP.SetSelected` (`|GetArrayItem` (`self.HexFields`) _index) true)
  (return))

(fn `changes`
  (locals (emptyCountInCols :type "Array of Integer") (randomType :type Integer))
  (bind _emptycountincols (`local.emptyCountInCols`))
  (bind _randomtype (`local.randomType`))
  (bind _boardfields (`self.boardFields`))
  (`KismetArrayLibrary.Array_Resize` _emptycountincols (`self.xElements`))
  (for _index (range (`self.yElements`))
    (for _index_2 (range (`self.xElements`))
      (bind _index_3 (`self.xy->index` _index_2 _index))
      (if (== (`|GetArrayItem` (`self.boardFields`) _index_3) -1)
        (bind _output (`|GetArrayItem` _emptycountincols _index_2))
        (`KismetArrayLibrary.Array_Set` _emptycountincols _index_2 (+ _output 1))
        (elif (> _output 0)
          (`self.swap` _index_3 (- _index_3 (* _output (`self.xElements`)))) ; dropping down element from high index to low index
        ))))
  (for (_array_element _array_index) _boardfields
    (if (== _array_element -1)
      (set `local.randomType` (`KismetMathLibrary.RandomInteger` (- (`self.typesNumber`) 1)))
      (`StaticMeshComponent.SetStaticMesh` (`|GetArrayItem` (`self.fieldsMeshes`) _array_index) (`|GetArrayItem` (`self.StaticSphereMeshes`) _randomtype))
      (`KismetArrayLibrary.Array_Set` _boardfields _array_index _randomtype))))

(fn `endField`
  (locals (change :type Boolean))
  (bind _selectedindexes (`self.selectedIndexes`))
  (bind _selectedindexes_2 (`self.selectedIndexes`))
  (set `local.change` (>= (`KismetArrayLibrary.Array_Length` _selectedindexes) 3))
  (for _array_element _selectedindexes
    (`/HexBlocksGame/hexFieldBP.SetSelected` (`|GetArrayItem` (`self.HexFields`) _array_element) false)
    (if (`local.change`)
      (`StaticMeshComponent.SetStaticMesh` (`|GetArrayItem` (`self.fieldsMeshes`) _array_element) null)
      (`KismetArrayLibrary.Array_Set` (`self.boardFields`) _array_element -1) ; -1 empty
    ))
  (if (`local.change`)
    (`self.changes`)
    (`/HexBlocksGame/Blueprints/BlocksPlayerController_BP.moveComplete` (cast `/HexBlocksGame/Blueprints/BlocksPlayerController_BP` (`GameplayStatics.GetPlayerController` 0) :!pure true) (`KismetArrayLibrary.Array_Length` _selectedindexes_2))
    (`GameplayStatics.PlaySound2D` (`self.CrossSound`) 1.0 1.0 0.0 null null))
  (`KismetArrayLibrary.Array_Clear` _selectedindexes_2)
  (set `self.selectingEnable` false)
  (`InstancedStaticMeshComponent.ClearInstances` (`self.Bridges`)))

(fn `isAdjacent`
  (params (x :type Integer) (y :type Integer))
  (returns (ReturnValue :type Boolean))
  (locals (tempArr :type "Array of Integer") (ParityOdd :type Boolean :default false) (XValue :type Integer) (Yvalue :type Integer))
  (set `local.ParityOdd` (!= (mod (`self.lastX`) 2) 0))
  (for _index (range 6)
    (set `local.XValue` (+ (`|GetArrayItem` (`self.maskX`) _index) (`self.lastX`)))
    (set `local.Yvalue` (+ (select `bool` (`local.ParityOdd`) :`false` (`|GetArrayItem` (`self.maskY1`) _index) :`true` (`|GetArrayItem` (`self.maskY2`) _index)) (`self.lastY`)))
    (`KismetArrayLibrary.Array_Add` (`local.tempArr`) (`self.xy->index` (`local.XValue`) (`local.Yvalue`))))
  (return (`KismetArrayLibrary.Array_Contains` (`local.tempArr`) (`self.xy->index` x y))))

(fn `selectField`
  (params (x :type Integer) (y :type Integer))
  (locals (indexFound :type Integer) (last_element :type Integer))
  (bind _index (`self.xy->index` x y))
  (bind _selectedindexes (`self.selectedIndexes`))
  (bind _selectedindexes_2 (`self.selectedIndexes`))
  (bind _selectedindexes_3 (`self.selectedIndexes`))
  (bind _selectedindexes_4 (`self.selectedIndexes`))
  (bind _last_element (`local.last_element`))
  (bind _returnvalue (`KismetArrayLibrary.Array_Length` _selectedindexes_4))
  (bind (_x _y) (`self.index->xy` (`|GetArrayItem` _selectedindexes_3 (- (`KismetArrayLibrary.Array_Length` _selectedindexes_3) 1))))
  (if (`KismetArrayLibrary.Array_Contains` _selectedindexes _index)
    (set `local.indexFound` (`KismetArrayLibrary.Array_Find` _selectedindexes _index))
    (set `local.last_element` (- (`KismetArrayLibrary.Array_Length` _selectedindexes) 1))
    (while (> _last_element (`local.indexFound`))
      (`/HexBlocksGame/hexFieldBP.SetSelected` (`|GetArrayItem` (`self.HexFields`) (`|GetArrayItem` _selectedindexes_2 _last_element)) false)
      (`KismetArrayLibrary.Array_Remove` _selectedindexes_2 _last_element)
      (`InstancedStaticMeshComponent.RemoveInstance` (`self.Bridges`) (- _last_element 1)) ; remove bridge
      (`/Engine/EditorBlueprintResources/StandardMacros.DecrementInt` _last_element))
    (set `self.lastX` _x)
    (set `self.lastY` _y)
    (else
      (bind _returnvalue_2 (`self.isAdjacent` x y))
      (if (and (`self.selectingEnable`) (== (`self.selectedType`) (`|GetArrayItem` (`self.boardFields`) _index)) _returnvalue_2)
        (`self.addField` x y)
        (`self.addBridge` (`|GetArrayItem` _selectedindexes_4 (- _returnvalue 2)) (`|GetArrayItem` _selectedindexes_4 (- _returnvalue 1)))))))

(fn `SpawnBoard`
  (locals (HexLocation :type "Vector Structure" :default (0.0 0.0 0.0)) (randomType :type Integer :default 0))
  (for _index (range (`self.yElements`))
    (for _index_2 (range (`self.xElements`))
      (bind (_cordx _cordy) (`self.xy->cords` _index_2 _index))
      (bind _output_get (set `local.HexLocation` (`KismetMathLibrary.MakeVector` _cordx _cordy)))
      (bind _returnvalue (`|SpawnActorFromClass` "/HexBlocksGame/hexFieldBP.hexFieldBP_C" (`KismetMathLibrary.Conv_VectorToTransform` _output_get) "Undefined" "OverrideRootScale" self _index_2 _index null))
      (`KismetArrayLibrary.Array_Add` (`self.HexFields`) _returnvalue)
      (bind _output_get_2 (set `local.randomType` (`KismetMathLibrary.RandomInteger` (`self.typesNumber`))))
      (`KismetArrayLibrary.Array_Add` (`self.boardFields`) _output_get_2)
      (bind _returnvalue_2 (`AddComponent|NODE_AddStaticMeshComponent-0` :`bManualAttachment` true :`RelativeTransform` (`KismetMathLibrary.MakeTransform` (+ (`local.HexLocation`) (199.699997 115.300049 -50.0)) (struct) (1.3 1.3 1.3))))
      (`KismetArrayLibrary.Array_Add` (`self.fieldsMeshes`) _returnvalue_2)
      (`StaticMeshComponent.SetStaticMesh` _returnvalue_2 (`|GetArrayItem` (`self.StaticSphereMeshes`) (`local.randomType`))))))

(fn `startField`
  (params (x :type Integer) (y :type Integer))
  (set `self.selectedType` (`|GetArrayItem` (`self.boardFields`) (`self.xy->index` x y)))
  (set `self.selectingEnable` true)
  (`self.addField` x y))

(fn `swap`
  (params (indexFrom :type Integer) (indexTo :type Integer))
  (locals (tempField :type "StaticMeshComponent Object Reference") (tempLocation :type "Vector Structure") (tempValue :type Integer))
  (bind _fieldsmeshes (`self.fieldsMeshes`))
  (bind _boardfields (`self.boardFields`))
  (bind _output (`|GetArrayItem` _fieldsmeshes indexFrom))
  (bind _output_2 (`|GetArrayItem` _fieldsmeshes indexTo))
  (set `local.tempField` _output)
  (set `local.tempLocation` (`SceneComponent.RelativeLocation` _output))
  (set `local.tempValue` (`|GetArrayItem` _boardfields indexFrom))
  (`SceneComponent.K2_SetRelativeLocation` _output (`SceneComponent.RelativeLocation` _output_2) false false) ; from = to
  (`SceneComponent.K2_SetRelativeLocation` _output_2 (`local.tempLocation`) false false) ; to= from
  (`KismetArrayLibrary.Array_Set` _fieldsmeshes indexFrom _output_2) ; from = to
  (`KismetArrayLibrary.Array_Set` _fieldsmeshes indexTo (`local.tempField`)) ; from = to
  (`KismetArrayLibrary.Array_Set` _boardfields indexFrom (`|GetArrayItem` _boardfields indexTo)) ; from = to
  (`KismetArrayLibrary.Array_Set` _boardfields indexTo (`local.tempValue`)) ; to = from
)

(fn `UserConstructionScript`
  (locals (randomType :type Integer)))