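; Hex tile actor for a board, identified by X and Y coordinates, that reports mouse input to its owning boardActor_BP.
; Hovering the mesh calls SelectField on the board and clicking calls StartField.
; The construction script creates a dynamic M_hex material instance tinted with the start color, and SetSelected switches that color to the highlight color and back.
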(event `self.StaticMesh.OnBeginCursorOver`
  (params (TouchedComponent :type "PrimitiveComponent Object Reference"))
  (`/HexBlocksGame/boardActor_BP.selectField` (cast `/HexBlocksGame/boardActor_BP` (`self.GetOwner`) :!pure true) (`self.x`) (`self.y`)))

(event `self.StaticMesh.OnClicked`
  (params (TouchedComponent :type "PrimitiveComponent Object Reference") (ButtonPressed :type "Key Structure"))
  (`/HexBlocksGame/boardActor_BP.startField` (cast `/HexBlocksGame/boardActor_BP` (`self.GetOwner`) :!pure true) (`self.x`) (`self.y`)))

(fn `SetSelected`
  (params (isSelected :type Boolean))
  (`MaterialInstanceDynamic.SetVectorParameterValue` (`self.dyn_material`) "color" (select `bool` isSelected :`false` (`self.start_color`) :`true` (`self.highlight_color`))))

(fn `UserConstructionScript`
  (bind _returnvalue (`KismetMaterialLibrary.CreateDynamicMaterialInstance` "/HexBlocksGame/Materials/M_hex.M_hex"))
  (set `self.dyn_material` _returnvalue)
  (`MaterialInstanceDynamic.SetVectorParameterValue` _returnvalue "color" (`self.start_color`))
  (`PrimitiveComponent.SetMaterial` (`self.StaticMesh`) 0 _returnvalue))