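; Player controller for a hex-collecting board game that tracks score and remaining moves.
; It spawns a camera on begin play, then GameStart resets state, moves the camera, enables click events and shows the game widget.
; Releasing left mouse calls EndField on every Blueprint and C++ board actor.
; Completed moves add the squared hex count to score; running out of moves swaps to the end-game widget.
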(event `Key|LeftMouseButton`
  (params (Key :type "Key Structure"))
  (:`Released`
    (`|ExecutionSequence`
      (:`then_0`
        ;[1 1 1] BLUEPRINTS
        (bind _outactors (`GameplayStatics.GetAllActorsOfClass` "/HexBlocksGame/boardActor_BP.boardActor_BP_C"))
        (for _array_element _outactors
          (`/HexBlocksGame/boardActor_BP.endField` _array_element)))
      (:`then_1`
        ;[1 1 1] C++
        (bind _outactors_2 (`GameplayStatics.GetAllActorsOfClass` "/Script/HexBlocksGame.BoardActor"))
        (for _array_element_2 _outactors_2
          (`BoardActor.endField` _array_element_2))))))

(event `self.ReceiveBeginPlay`
  (bind _returnvalue (`|SpawnActorFromClass` "/Script/Engine.CameraActor" (`self.cameraStartTransform`) "Undefined" "OverrideRootScale" null null))
  (set `self.cameraC` _returnvalue)
  (`self.SetViewTargetWithBlend` _returnvalue))

(event `self.moveCompleted`
  (params (numberHexesCollected :type Integer))
  (`self.moveComplete` numberHexesCollected))

(fn `gameEnd`
  (set `self.bEnableClickEvents` false)
  (`WidgetLayoutLibrary.RemoveAllWidgets`)
  (bind _returnvalue (`|CreateWidget` "/HexBlocksGame/endGameWidget.endGameWidget_C"))
  (`UserWidget.AddToViewport` _returnvalue 0))

(fn `gameStart`
  (set `self.score` 0)
  (set `self.moves` 10)
  (set `self.bEnableClickEvents` true)
  (`self.K2_SetActorTransform` (`self.cameraC`) (`self.cameraGameTransform`) false false)
  (bind _returnvalue (`|CreateWidget` "/HexBlocksGame/gameWidget.gameWidget_C"))
  (`UserWidget.AddToViewport` _returnvalue 0))

(fn `moveComplete`
  (params (numberOfHexes :type Integer))
  (bind _moves (`self.moves`))
  (set `self.score` (+ (`self.score`) (* numberOfHexes numberOfHexes)))
  (`/Engine/EditorBlueprintResources/StandardMacros.DecrementInt` _moves
    (:`  `
      (if (<= _moves 0)
        (`self.gameEnd`)))))

(fn `UserConstructionScript`)